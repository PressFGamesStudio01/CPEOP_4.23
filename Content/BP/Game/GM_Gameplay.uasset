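; Gameplay game mode that procedurally builds a linear stage along X when play begins.
; It repeats the placed Land_M tile's class up to its set distance, adds a finish, and creates the progress widget.
; It spaces four guardian gates (mini-bosses, then a level-specific boss) and level-specific enemy spawners along the track, then spawns and possesses the hero.
; StageFinished shows results and destroys remaining enemies.
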(event `self.ReceiveBeginPlay`
  (bind _asmy_gins (cast `/Game/BP/Game/MyGIns` (`GameplayStatics.GetGameInstance`)))
  (set `self.GameIns` _asmy_gins)
  (if true
    (`self.Init01`)))

(event `Init01`
  ;[1 1 1 1 24] Level Initialization
  (`self.GenerateLevel`)
  (`self.LevelProgress`)
  (`self.SpawnEnemy`)
  (`self.SpawnHero`)
  (`self.SetFinishLocation`))

(event `StageFinished`
  ;[1 1 1] On Stage Finished
  ;;[1 1 1] Show Results Widget
  (`/Game/BP/Game/MyGIns.W_StageResults` (`self.GameIns`))
  ;;[1 1 1] Remove All Enemys
  (bind _outactors (`GameplayStatics.GetAllActorsOfClass` "/Game/BP/Character/Enemy/MEnemy.MEnemy_C"))
  (for _array_element _outactors
    (`/Engine/EditorBlueprintResources/StandardMacros.IsValid` _array_element
      (:`Is Valid`
        (`self.K2_DestroyActor`)))))

(event `GenerateLevel`
  ;[1 1 1 1 24] Level Initialization
  ;;[1 1 1] Check Enemy spawners and Start Scene Generation
  (bind _outactors (`GameplayStatics.GetAllActorsOfClass` "/Game/BP/LevelBP/Land_M.Land_M_C"))
  (bind _output (`|GetArrayItem` _outactors))
  (`/Engine/EditorBlueprintResources/StandardMacros.IsValid` _output
    (:`Is Valid`
      (set `self.LastLocation` (`self.K2_GetActorLocation` _output))
      (set `self.LandClass` (`GameplayStatics.GetObjectClass` _output))
      (set `self.EnSpawners` (`/Game/BP/LevelBP/Land_M.Enemys` _output))
      (`self.SpawnLP` (`/Game/BP/LevelBP/Land_M.Dist` _output) (`/Game/BP/LevelBP/Land_M.Size` _output)))))

(event `SpawnLP`
  (params (dist :type "Float (double-precision)") (size :type "Float (double-precision)"))
  (bind (_lastlocation_x _lastlocation_y _lastlocation_z) (`KismetMathLibrary.BreakVector` (`self.LastLocation`)))
  ;[1 1 1 1 24] Level Initialization
  ;;[1 1 1] Check Enemy spawners and Start Scene Generation
  ;;;[1 1 1] Land generator with loop
  (`|ExecutionSequence`
    (:`then_0`
      (set `self.DistToFinish` dist)
      (for _index (range 1 (+ (+ (`KismetMathLibrary.FTrunc` (/ dist size)) 1) 1))
        (`|SpawnActorFromClass` (`self.LandClass`) (`KismetMathLibrary.MakeTransform` (`KismetMathLibrary.MakeVector` (+ _lastlocation_x (* size (`KismetMathLibrary.Conv_IntToDouble` _index))) _lastlocation_y _lastlocation_z)) "AlwaysSpawn" "OverrideRootScale" null null))
      (`|SpawnActorFromClass` "/Game/BP/LevelBP/BP_Finish.BP_Finish_C" (`KismetMathLibrary.MakeTransform` (`KismetMathLibrary.MakeVector` (`self.DistToFinish`))) "Undefined" "OverrideRootScale" null self null))))

(event `LevelProgress`
  ;[1 1 1 1 24] Level Initialization
  ;;[1 1 1] Create Level Progress widget
  (bind _returnvalue (`|CreateWidget` "/Game/BP/UI/Game/LevelProgress.LevelProgress_C"))
  (`UserWidget.AddToViewport` _returnvalue -1))

(event `SpawnEnemy`
  ;[1 1 1 1 24] Level Initialization
  ;;[1 1 1] Spawn Enemy's Spawners
  (`self.Spawn Bosses`)
  (`self.SpawnEn`))

(event `SpawnEn`
  (bind _enspawners (`self.EnSpawners`))
  ;[1 1 1 1 24] Level Initialization
  ;;[1 1 1] Spawn Enemy's Spawners
  (for _index (range 1 (+ _enspawners 1))
    (bind _output_get (set `self.EnSpawnerClass` (select `int` (`/Game/BP/Game/MyGIns.LevelProgress` (`self.GameIns`)) :`0` "/Game/BP/LevelBP/EnSpawners/EnSpawn_01.EnSpawn_01_C" :`1` "/Game/BP/LevelBP/EnSpawners/EnSpawn_02.EnSpawn_02_C" :`2` "/Game/BP/LevelBP/EnSpawners/EnSpawn_03.EnSpawn_03_C" :!type "/Game/BP/LevelBP/EnSpawner Class Reference")))
    (`|SpawnActorFromClass` :`Class` _output_get :`SpawnTransform` (`KismetMathLibrary.MakeTransform` (`KismetMathLibrary.MakeVector` (+ (* (/ (- (`self.DistToFinish`) (`self.StartLocation`)) (`KismetMathLibrary.Conv_IntToDouble` _enspawners)) (`KismetMathLibrary.Conv_IntToDouble` _index)) (`self.StartLocation`) -300.0) 0.0 60.0) (struct :`Yaw` 180.0)) :`CollisionHandlingOverride` "AlwaysSpawn" :`TransformScaleMethod` "OverrideRootScale" :`Quantity` (`KismetMathLibrary.RandomIntegerInRange` 2 4) :`Dist` 250.0 :`Instigator` null)))

(event `Spawn Bosses`
  (bind _minibosses (`self.MiniBosses`))
  (bind _gameins (`self.GameIns`))
  ;[1 1 1 1 24] Level Initialization
  ;;[1 1 1] Spawn Enemy's Spawners
  (for _index (range 1 5)
    (`|SpawnActorFromClass` "/Game/BP/LevelBP/Barrier_Gate.Barrier_Gate_C" (`KismetMathLibrary.MakeTransform` (`KismetMathLibrary.MakeVector` (+ (* (/ (- (`self.DistToFinish`) (`self.StartLocation`)) 4.0) (`KismetMathLibrary.Conv_IntToDouble` _index)) (`self.StartLocation`)) 0.0 300.0)) "Undefined" "OverrideRootScale" null (`self.Player`) (select `bool` (== _index 4) :`false` (`|GetArrayItem` _minibosses (`KismetMathLibrary.RandomIntegerInRange` 0 (`KismetArrayLibrary.Array_Length` _minibosses))) :`true` (`|GetArrayItem` (`self.Bosses`) (`/Game/BP/Game/MyGIns.LevelProgress` (`self.GameIns`)))) _gameins (+ (`/Game/BP/Game/MyGIns.LevelProgress` _gameins) 4) null)))

(event `SpawnHero`
  ;[1 1 1 1 24] Level Initialization
  ;;[1 1 1] Spawn Hero
  (if true
    (bind _returnvalue (`|SpawnActorFromClass` "/Game/BP/Character/Player/p1.p1_C" (`KismetMathLibrary.MakeTransform` (0.0 100.0 100.0)) "AdjustIfPossibleButAlwaysSpawn" "OverrideRootScale" null 1 null))
    (`Controller.Possess` (`GameplayStatics.GetPlayerController` 0) _returnvalue)
    (`/Game/BP/Game/MyGIns.w_TouchScreen` (`self.GameIns`) _returnvalue)))

(event `SetFinishLocation`
  ;[1 1 1 1 24] Level Initialization
)

(fn `UserConstructionScript`)