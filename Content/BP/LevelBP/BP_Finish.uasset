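; Stage finish trigger actor that ends the stage when the player reaches it.
; Its Box overlap calls StageFinished on GameModeRef when the other actor is player character 0.
; On BeginPlay it destroys itself if GameModeRef is invalid, otherwise it caches the MyGIns game instance, which is not used further here.
; GameModeRef is not assigned anywhere in these graphs.
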(event `self.ReceiveBeginPlay`
  (if (`KismetSystemLibrary.IsValid` (`self.GameModeRef`))
    (bind _asmy_gins (cast `/Game/BP/Game/MyGIns` (`GameplayStatics.GetGameInstance`)))
    (set `self.GameInsRef` _asmy_gins)
    (else
      (`self.K2_DestroyActor`))))

(event `self.Box.OnComponentBeginOverlap`
  (params (OverlappedComponent :type "PrimitiveComponent Object Reference") (OtherActor :type "Actor Object Reference") (OtherComp :type "PrimitiveComponent Object Reference") (OtherBodyIndex :type Integer) (bFromSweep :type Boolean) (SweepResult :type "HitResult Structure (by ref)"))
  (if (== OtherActor (`GameplayStatics.GetPlayerCharacter` 0))
    (`/Game/BP/Game/GM_Gameplay.StageFinished` (`self.GameModeRef`))))

(fn `UserConstructionScript`)